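; Tent_BP is a placeholder tent actor that triggers the fail endgame when the player character enters it.
; When TopDownCharacterBoi overlaps EnterBox, it pauses the game, shows the EndgameFail widget, switches input to UI only and shows the mouse cursor.
; An older pause-UI branch and an optional attenuated clown soundtrack at the tent are left disconnected.
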(event `self.ReceiveBeginPlay`)

(event `self.EnterBox.OnComponentBeginOverlap`
  (params (OverlappedComponent :type "PrimitiveComponent Object Reference") (OtherActor :type "Actor Object Reference") (OtherComp :type "PrimitiveComponent Object Reference") (OtherBodyIndex :type Integer) (bFromSweep :type Boolean) (SweepResult :type "HitResult Structure (by ref)"))
  (bind _returnvalue (`GameplayStatics.GetPlayerController` 0))
  (cast `/Game/Toms_shit/TopDownCharacterBoi` OtherActor)
  (`GameplayStatics.SetGamePaused` true)
  (bind _returnvalue_2 (`|CreateWidget` "/Game/Sandrine/UI/In-Game/Endgame-Fail.Endgame-Fail_C"))
  (`UserWidget.AddToViewport` _returnvalue_2 0)
  (`WidgetBlueprintLibrary.SetInputMode_UIOnlyEx` _returnvalue null)
  (set `PlayerController.bShowMouseCursor` true _returnvalue)
  (set `self.WasPaused` true))

(fn `UserConstructionScript`)