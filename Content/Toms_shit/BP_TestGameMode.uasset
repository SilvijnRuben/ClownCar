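; BP_TestGameMode is a game mode that runs a minute-and-second countdown and ends the game when it expires.
; BeginPlay shows the Countdown widget, and Tick uses a one-second Delay as a throttle to decrement the time.
; At zero it pauses the game and shows the EndGame widget.
; An unconnected count-up timer chain also remains in the event graph.
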(event `self.ReceiveBeginPlay`
  ;[1 1 1] Timer UI
  (bind _returnvalue (`|CreateWidget` "/Game/Sandrine/UI/In-Game/Countdown.Countdown_C"))
  (`UserWidget.AddToViewport` _returnvalue 0))

(event `self.ReceiveTick`
  (params (DeltaSeconds :type "Float (single-precision)"))
  ;[1 1 1] Countdown Logic
  (`KismetSystemLibrary.Delay` 1.0)
  (set `self.Countdown-Sec` (- (`self.Countdown-Sec`) 1))
  (if (< (`self.Countdown-Sec`) 0)
    (set `self.Countdown-Min` (- (`self.Countdown-Min`) 1))
    (set `self.Countdown-Sec` 59))
  (if (== (`self.Countdown-Sec`) 0)
    (if (== (`self.Countdown-Min`) 0)
      (`GameplayStatics.SetGamePaused` true)
      (bind _returnvalue (`|CreateWidget` "/Game/Sandrine/UI/In-Game/EndGame.EndGame_C" (`GameplayStatics.GetPlayerController` 0)))
      (`UserWidget.AddToViewport` _returnvalue 0))))

(fn `UserConstructionScript`)