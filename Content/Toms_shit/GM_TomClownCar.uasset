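; Game mode for the clown car level that runs a timed challenge with a failure screen.
; BeginPlay locks player input during a honking 3-2-1-Go widget, then shows the countdown UI and starts music.
; Tick uses Delay nodes to decrement the clock each second, pausing on the EndGameFail widget at zero.
; AnnounceClownCollected relays to CallClownCollected, and a count-up timer is left disconnected.
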(event `self.ReceiveBeginPlay`
  (bind _returnvalue (`GameplayStatics.GetPlayerCharacter` 0))
  (bind _returnvalue_2 (`GameplayStatics.GetPlayerController` 0))
  (`self.DisableInput` _returnvalue _returnvalue_2)
  (`|ExecutionSequence`
    (:`then_0`
      (bind _returnvalue_3 (`|CreateWidget` "/Game/Sandrine/UI/321Go.321Go_C"))
      (`UserWidget.AddToViewport` _returnvalue_3 0)
      (`KismetSystemLibrary.Delay` 3.0)
      (`Widget.RemoveFromParent` _returnvalue_3)
      (`self.EnableInput` _returnvalue _returnvalue_2)
      (`GameplayStatics.PlaySound2D` "/Game/Sandrine/Sounds/UI-UX/CheerfulHorn1.CheerfulHorn1" 1.0 1.0 0.0 null null)
      ;[1 1 1] Timer UI
      (bind _returnvalue_4 (`|CreateWidget` "/Game/Sandrine/UI/In-Game/Countdown.Countdown_C"))
      (`UserWidget.AddToViewport` _returnvalue_4 0)
      (`KismetSystemLibrary.Delay` 1.5)
      (`GameplayStatics.PlaySound2D` "/Game/Sandrine/Sounds/MisterClownSoundtrack_Cue.MisterClownSoundtrack_Cue" 1.0 1.0 0.0 null null))
    (:`then_1`
      (`GameplayStatics.PlaySound2D` "/Game/Sandrine/Sounds/UI-UX/Menu-HoverHonk_Cue.Menu-HoverHonk_Cue" 1.0 1.0 0.0 null null)
      (`KismetSystemLibrary.Delay` 1.0)
      (`GameplayStatics.PlaySound2D` "/Game/Sandrine/Sounds/UI-UX/Menu-HoverHonk_Cue.Menu-HoverHonk_Cue" 1.0 1.0 0.0 null null)
      (`KismetSystemLibrary.Delay` 1.0)
      (`GameplayStatics.PlaySound2D` "/Game/Sandrine/Sounds/UI-UX/Menu-HoverHonk_Cue.Menu-HoverHonk_Cue" 1.0 1.0 0.0 null null)
      (`KismetSystemLibrary.Delay` 1.0))))

(event `self.ReceiveTick`
  (params (DeltaSeconds :type "Float (single-precision)"))
  (bind _returnvalue (`GameplayStatics.GetPlayerController` 0))
  (`KismetSystemLibrary.Delay` 1.0)
  (set `self.3210` (- (`self.3210`) 1))
  ;[1 1 1] Countdown Logic
  (`KismetSystemLibrary.Delay` 1.0)
  (set `self.Countdown-Sec` (- (`self.Countdown-Sec`) 1))
  (if (< (`self.Countdown-Sec`) 0)
    (set `self.Countdown-Min` (- (`self.Countdown-Min`) 1))
    (set `self.Countdown-Sec` 59))
  (if (== (`self.Countdown-Sec`) 0)
    (if (== (`self.Countdown-Min`) 0)
      (bind _returnvalue_2 (`|CreateWidget` "/Game/Sandrine/UI/In-Game/EndGame-Fail.EndGame-Fail_C" _returnvalue))
      (`WidgetBlueprintLibrary.SetInputMode_UIOnlyEx` _returnvalue _returnvalue_2)
      (set `PlayerController.bShowMouseCursor` true _returnvalue)
      (`UserWidget.AddToViewport` _returnvalue_2 0)
      (`GameplayStatics.SetGamePaused` true)
      (`GameplayStatics.PlaySound2D` "/Game/Sandrine/Sounds/UI-UX/Descend_Cue.Descend_Cue" 1.0 1.0 0.0 null null))))

(event `Announce Clown Collected`
  (`self.Clown Collected`))

(fn `UserConstructionScript`)