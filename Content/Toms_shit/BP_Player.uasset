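; Player character that constantly accelerates forward and is steered only with left and right turn inputs.
; Each Tick ramps acceleration and turn rate to their caps, rotates yaw by the summed input direction, then overwrites CharacterMovement velocity.
; Curves over normalized turn rate shape turning speed and velocity damping, with forward thrust added every frame without delta-time scaling.
; Turn rate resets when steering is neutral; ResetSpeeds zeroes acceleration but is not called here.
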(event `self.ReceiveTick`
  (params (DeltaSeconds :type "Float (single-precision)"))
  (`self.UpdateSpeeds` DeltaSeconds)
  (`self.Update Turn` DeltaSeconds)
  (`self.Move` DeltaSeconds))

(event `InputAction|TurnLeft`
  (params (Key :type "Key Structure"))
  (:`Pressed`
    (`self.Turn` -1 :!label _label))
  (:`Released`
    (`self.Turn` 1 :!label _label_2)))

(event `InputAction|TurnRIght`
  (params (Key :type "Key Structure"))
  (:`Pressed`
    (goto _label_2))
  (:`Released`
    (goto _label)))

(fn `Move`
  (params (DeltaTime :type "Float (double-precision)"))
  (bind _charactermovement (`self.CharacterMovement`))
  (set `MovementComponent.Velocity` (+ (* (`MovementComponent.Velocity` _charactermovement) (- 1.0 (`CurveFloat.GetFloatValue` (`self.DellerationCurve`) (/ (`self.CurrentTurnRate`) (`self.MaxTurnRate`))))) (* (`KismetMathLibrary.GetForwardVector` (`KismetMathLibrary.MakeRotator` 0.0 0.0 (.yaw (`self.K2_GetActorRotation`)))) (`self.Accelleration`))) _charactermovement))

(fn `ResetSpeeds`
  (set `self.Accelleration` 0.0))

(fn `Turn`
  (params (Direction :type Integer))
  (set `self.TurnDirection` (+ (`self.TurnDirection`) Direction)))

(fn `Update Turn`
  (params (DeltaTime :type "Float (double-precision)"))
  (bind _maxturnrate (`self.MaxTurnRate`))
  (`self.K2_SetActorRotation` (`KismetMathLibrary.MakeRotator` (.roll (`self.K2_GetActorRotation`)) (.pitch (`self.K2_GetActorRotation`)) (+ (* (`self.TurnDirection`) (* DeltaTime (* (`CurveFloat.GetFloatValue` (`self.TurnRateCurve`) (/ (`self.CurrentTurnRate`) _maxturnrate)) _maxturnrate))) (.yaw (`self.K2_GetActorRotation`))))))

(fn `UpdateSpeeds`
  (params (DeltaTime :type "Float (double-precision)"))
  (set `self.Accelleration` (`KismetMathLibrary.FMin` (+ (* (`self.AccellerationRate`) DeltaTime) (`self.Accelleration`)) (`self.MaxAccellation`)))
  (set `self.CurrentTurnRate` (`KismetMathLibrary.SelectFloat` 0.0 (`KismetMathLibrary.FMin` (+ (`self.CurrentTurnRate`) (* (`self.TurnRateAccelleration`) DeltaTime)) (`self.MaxTurnRate`)) (== (`self.TurnDirection`) 0))))

(fn `UserConstructionScript`)