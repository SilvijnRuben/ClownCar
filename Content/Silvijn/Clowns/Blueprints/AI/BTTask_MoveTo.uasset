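; Behavior tree task that moves the AI-controlled clown to a location read from a Blackboard vector key.
; It runs an async AI MoveTo and passes its outcome through a collapsed Notify Movement graph, which tells BP_Clown when movement begins.
; Success also signals the clown that movement ended, while failure skips that call.
; Both outcomes finish the task with the matching success flag.
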(event `self.ReceiveExecuteAI`
  (params (OwnerController :type "AIController Object Reference") (ControlledPawn :type "Pawn Object Reference"))
  (bind _output_get (set `self.ControlledPawn` ControlledPawn))
  (bind _movementresult (`|AIMoveTo` _output_get (`BTFunctionLibrary.GetBlackboardValueAsVector` (`self.MoveToKey`)) null)
    (:`then`
      (bind _succeeded (`self.Notify Movement` _movementresult :!label _label)
        (:`Finish`
          (`self.FinishExecute` _succeeded))))
    (:`OnSuccess`
      (goto _label :!via `Succes`))
    (:`OnFail`
      (goto _label :!via `Fail`))))