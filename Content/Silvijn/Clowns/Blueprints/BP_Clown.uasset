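; BP_Clown is an AI character that can be knocked rolling, flee and be collected.
; A hit pauses its AI, launches it with physics and wig particles, and sends overlapping clowns fleeing along a navigation raycast, before a timer stands it up.
; Collection uses a timeline to shrink it toward TopDownCharacterBoi, then notifies BP_ClownSpawner and destroys it.
; Walk speed is randomized, and a looping timer spins the mesh in steps during movement.
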(event `self.ReceiveBeginPlay`
  (set `CharacterMovementComponent.MaxWalkSpeed` (`KismetMathLibrary.RandomFloatInRange` 600.0 700.0) (`self.CharacterMovement`)))

(event `Begin Movement`
  (bind _returnvalue (`KismetSystemLibrary.K2_SetTimerDelegate` (delegate `Rotate Clown`) 0.2 true))
  (set `self.MovementTimer` _returnvalue))

(event `Rotate Clown`
  (`SceneComponent.K2_AddLocalRotation` (`self.Mesh`) (struct :`Pitch` -90.0) false true))

(event `End Movement`
  (`KismetSystemLibrary.K2_ClearAndInvalidateTimerHandle` (`self.MovementTimer`)))

(event `Run Away`
  (params (CarHitLoc :type "Vector Structure"))
  (bind _returnvalue (`self.K2_GetActorLocation`))
  (`self.Stop AI Logic`)
  (`self.Reset Rotations`)
  (bind _hitlocation (`NavigationSystemV1.NavigationRaycast` _returnvalue (* (`KismetMathLibrary.GetDirectionUnitVector` CarHitLoc _returnvalue) 100000.0) null null))
  (`|AIMoveTo` self _hitlocation null
    (:`OnSuccess`
      (`self.Reset Rotations`)
      (`self.Restart AI Logic`))))

(event `Clown Hit`
  (params (`Hit Normal` :type "Vector Structure"))
  (if (not (`self.BeingCollected`))
    (set `self.HitNormal` `Hit Normal`)
    (`PrimitiveComponent.SetCollisionEnabled` (`self.RollSphere`) "QueryAndPhysics")
    (`PrimitiveComponent.SetCollisionEnabled` (`self.CapsuleComponent`) "QueryAndPhysics")
    (`PrimitiveComponent.SetSimulatePhysics` (`self.CapsuleComponent`) true)
    (`PrimitiveComponent.AddForce` (`self.RollSphere`) (* (`self.HitNormal`) (`self.RollAwayModifier`)) "None" true)
    (`self.Stop AI Logic`)
    (`self.End Movement`)
    (`KismetSystemLibrary.K2_SetTimerDelegate` (delegate `Stand Up`) 2.0)
    (`NiagaraFunctionLibrary.SpawnSystemAtLocation` "/Game/Geometry/clownB/PS_WigSystem.PS_WigSystem" (`SceneComponent.K2_GetComponentLocation` (`self.ClownMesh`)))
    (`self.Warn Surrounding Clowns`)))

(event `Stand Up`
  (`PrimitiveComponent.SetCollisionEnabled` (`self.RollSphere`) "NoCollision")
  (`PrimitiveComponent.SetSimulatePhysics` (`self.CapsuleComponent`) false)
  (`self.Reset Rotations`)
  (`self.Restart AI Logic`))

(event `Get Collected`
  (bind _returnvalue (`self.K2_GetActorLocation`))
  (set `self.BeingCollected` true)
  (`self.Stop AI Logic`)
  (`self.SetActorEnableCollision` false)
  (bind (_direction _shrink) (`Timeline|Shrink Timeline`)
    (:`Update`
      (`self.SetActorScale3D` (`KismetMathLibrary.Conv_DoubleToVector` _shrink))
      (bind _returnvalue_2 (`GameplayStatics.GetActorOfClass` "/Game/Toms_shit/TopDownCharacterBoi.TopDownCharacterBoi_C"))
      (`self.K2_SetActorLocation` (+ _returnvalue (* (- (`self.K2_GetActorLocation` _returnvalue_2) _returnvalue) (* _shrink 0.5)))))
    (:`Finished`
      (bind _returnvalue_3 (`GameplayStatics.GetActorOfClass` "/Game/Silvijn/Clowns/Blueprints/BP_ClownSpawner.BP_ClownSpawner_C"))
      (`/Game/Silvijn/Clowns/Blueprints/BP_ClownSpawner.Clown Killed` _returnvalue_3)
      (`self.K2_DestroyActor`))))

(fn `UserConstructionScript`)