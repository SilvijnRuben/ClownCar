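; BP_ClownSpawner is an actor that spawns a capped number of clowns over time, starting at BeginPlay.
; A Loop with Delay macro fires once per iteration, waiting SpawnDelay between spawns until MaxAmountClowns is reached.
; Each pass randomly picks one of the first two Clowns classes and spawns it at a random navigable point within SpawnRadius of the spawner.
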(event `self.ReceiveBeginPlay`
  (`self.Loop with Delay` (`self.MaxAmountClowns`) (`self.SpawnDelay`)
    (:`true`
      (`|SpawnActorFromClass` (`|GetArrayItem` (`self.Clowns`) (`KismetMathLibrary.RandomIntegerInRange` 0 1)) (`KismetMathLibrary.MakeTransform` (`NavigationSystemV1.K2_GetRandomLocationInNavigableRadius` (`self.K2_GetActorLocation`) (`self.SpawnRadius`) null null)) "Undefined" "OverrideRootScale" null null))))

(fn `UserConstructionScript`)